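; Scatters fluorescent light fixture meshes at random over a grid centred on the actor.
; On BeginPlay it loops from negative to positive GridX and GridY, spacing cells by CellSizeX and CellSizeY, and fills each on a coin flip.
; Each filled cell adds matching instances to BaseLight and FluoTube with a fixed rotation and scale.
; The unseeded layout exists only at runtime, as the construction script is empty.
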(event EventBeginPlay
  (bind _gridx (Variables|Default|GetGridX))
  (bind _gridy (Variables|Default|GetGridY))
  (for _index (range (* _gridx -1) _gridx)
    (for _index_2 (range (* _gridy -1) _gridy)
      (if (Math|Random|RandomBool)
        (Components|InstancedStaticMesh|AddInstance (Variables|Default|GetBaseLight) (Math|Transform|MakeTransform (Math|Vector|MakeVector (* _index (Variables|Default|GetCellSizeX)) (* _index_2 (Variables|Default|GetCellSizeY)) 0.0) "180.000000,0.000000,0.000000" "2.000000,2.000000,2.000000") false)
        (Components|InstancedStaticMesh|AddInstance (Variables|Default|GetFluoTube) (Math|Transform|MakeTransform (Math|Vector|MakeVector (* _index (Variables|Default|GetCellSizeX)) (* _index_2 (Variables|Default|GetCellSizeY)) 0.0) "180.000000,0.000000,0.000000" "2.000000,2.000000,2.000000") false)))))

(fn ConstructionScript)