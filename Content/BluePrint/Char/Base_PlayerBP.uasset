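; Base player character with Enhanced Input movement, look and running, plus Escape to quit.
; A looping timer plays footstep sounds while moving on the ground, choosing the cue from a downward trace's physical surface.
; Running changes walk speed and restarts that timer at a different interval.
; Each tick adds a sine-based pitch and yaw camera bob, with amplitude and frequency clamped from velocity.
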(event Custom|FootStep
  ;[1 1 1] Footstep Temp
  (if (and (> (Math|Vector|VectorLength (Transformation|GetVelocity)) 5e+01) (not (AI|Components|NavMovement|IsFalling (Variables|Character|GetCharacterMovement))))
    (Audio|PlaySound2D (Utilities|Select :Index (CallFunction|CheckSurface) :SurfaceType_Default "/Game/Ultimate_SFX/Ultimate_Footstep_Sounds/Wav/CONCRETE/Concrete_footsteps_1_Cue.Concrete_footsteps_1_Cue" :SurfaceType1 "/Game/Ultimate_SFX/Ultimate_Footstep_Sounds/Wav/CONCRETE/Concrete_footsteps_1_Cue.Concrete_footsteps_1_Cue" :SurfaceType2 "/Game/Ultimate_SFX/Ultimate_Footstep_Sounds/Wav/DIRT/Barefoot_Dirt_footsteps_1_Cue.Barefoot_Dirt_footsteps_1_Cue") 0.5 1.0 0.0 0 0)))

(event Custom|FootstepLoop
  ;[1 1 1] Footstep Temp
  (bind _returnvalue (Utilities|Time|SetTimerbyEvent (delegate Custom|FootStep) (Variables|Default|GetFootStepTime) true))
  (Variables|Default|SetFootstepTimer _returnvalue))

(event Input|EnhancedActionEvents|EnhancedInputActionMove
  (params (ActionValue :type Vector%202D%20Structure) (ElapsedSeconds :type Float%20%28double-precision%29) (TriggeredSeconds :type Float%20%28double-precision%29) (InputAction :type Input%20Action%20Object%20Reference :default "/Game/BluePrint/Input/Move.Move"))
  (Pawn|Input|AddMovementInput (Transformation|GetActorRightVector) (.x ActionValue) false)
  (Pawn|Input|AddMovementInput (Transformation|GetActorForwardVector) (.y ActionValue) false))

(event Input|EnhancedActionEvents|EnhancedInputActionCamera_Move
  (params (ActionValue :type Vector%202D%20Structure) (ElapsedSeconds :type Float%20%28double-precision%29) (TriggeredSeconds :type Float%20%28double-precision%29) (InputAction :type Input%20Action%20Object%20Reference :default "/Game/BluePrint/Input/Camera_Move.Camera_Move"))
  (Pawn|Input|AddControllerPitchInput (.y ActionValue))
  (Pawn|Input|AddControllerYawInput (.x ActionValue)))

(event Input|EnhancedActionEvents|EnhancedInputActionRunning
  (params (ActionValue :type Boolean) (ElapsedSeconds :type Float%20%28double-precision%29) (TriggeredSeconds :type Float%20%28double-precision%29) (InputAction :type Input%20Action%20Object%20Reference :default "/Game/BluePrint/Input/Running.Running"))
  (bind _charactermovement (Variables|Character|GetCharacterMovement))
  (:Started
    (Variables|/Script/Engine.CharacterMovementComponent|SetMaxWalkSpeed _charactermovement 1.5e+03)
    (Utilities|Time|ClearandInvalidateTimerbyHandle (Variables|Default|GetFootstepTimer))
    (Variables|Default|SetFootStepTime 0.35)
    (CallFunction|FootstepLoop :!label _label))
  (:Completed
    (Variables|/Script/Engine.CharacterMovementComponent|SetMaxWalkSpeed _charactermovement 6e+02)
    (Utilities|Time|ClearandInvalidateTimerbyHandle (Variables|Default|GetFootstepTimer))
    (Variables|Default|SetFootStepTime 0.5)
    (goto _label)))

(event EventTick
  (params (DeltaSeconds :type Float%20%28single-precision%29))
  (CallFunction|MoveCamera))

(event EventBeginPlay
  (bind _returnvalue (Game|GetPlayerController 0))
  (bind _returnvalue_2 (PlayerController|LocalPlayerSubsystems|GetEnhancedInputLocalPlayerSubsystem _returnvalue))
  (Utilities|IsValid _returnvalue_2
    (:Is%20Valid
      (Input|AddMappingContext _returnvalue_2 "/Game/BluePrint/Input/PlayerInputBase.PlayerInputBase" 0 "(bIgnoreAllPressedKeysUntilRelease=True,bForceImmediately=False,bNotifyUserSettings=False)")
      (CallFunction|FootstepLoop))))

(event Input|KeyboardEvents|Escape
  (params (Key :type Key%20Structure :default "None"))
  (:Pressed
    (Game|QuitGame 0 "Quit" false)))

(fn ConstructionScript
  (|CallParentFunction))

(fn MoveCamera
  (bind (_amplitude _frequency) (CallFunction|GetSpeedVsCamMove))
  (Variables|Default|SetRuntime (+ (Utilities|Time|GetWorldDeltaSeconds) (Variables|Default|GetRuntime)))
  (Transformation|AddLocalRotation (Variables|Default|GetCamera) (Math|Rotator|MakeRotator 0.0 (CallFunction|SinMove _amplitude _frequency (Variables|Default|GetRuntime)) (CallFunction|SinMove (/ _amplitude 2.0) (/ _frequency 2.0) (Variables|Default|GetRuntime))) false false))

(fn GetSpeedVsCamMove
  (bind _returnvalue (Transformation|GetVelocity))
  (bind _returnvalue_2 (Math|Vector|VectorLength _returnvalue))
  (return (Math|Float|Clamp(Float) _returnvalue_2 0.02 0.08) (Math|Float|Clamp(Float) _returnvalue_2 2.0 18.0)))

(fn CheckSurface
  (bind _returnvalue (Transformation|GetActorLocation))
  (bind (_outhit _returnvalue_2) (Collision|LineTraceByChannel _returnvalue (+ _returnvalue "0.000000,0.000000,-150.000000") "TraceTypeQuery1" false 0 "None"))
  (if _returnvalue_2
    (return (Variables|/Script/PhysicsCore.PhysicalMaterial|GetSurfaceType (.PhysMat (Collision|BreakHitResult _outhit))))))