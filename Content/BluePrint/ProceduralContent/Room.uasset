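; Procedural room actor that builds a tile grid with floor, optional ceiling and perimeter walls, either in the construction script (PreLoad) or at BeginPlay.
; GenerateBaseRoom adds floor and ceiling mesh instances, then passes each edge segment to WallOrDoor, flagging door-eligible slots at a regular interval.
; WallOrDoor spawns and records a Door actor on a seeded random roll weighted by DoorCount and doors already placed, otherwise adding a wall instance.
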(event EventBeginPlay
  (if (not (Variables|Default|GetPreLoad?))
    (Utilities|Array|Clear (Variables|Default|GetDoors))
    (CallFunction|GenerateBaseRoom)))

(fn ConstructionScript
  (if (Variables|Default|GetPreLoad?)
    (Utilities|Array|Clear (Variables|Default|GetDoors))
    (CallFunction|GenerateBaseRoom)))

(fn GenerateBaseRoom
  (for _index (range 0 (- (Variables|Default|GetRoomTileY) 1))
    (for _index_2 (range 0 (- (Variables|Default|GetRoomTileX) 1))
      (Components|InstancedStaticMesh|AddInstance (Variables|Default|GetFloor) (Math|Transform|MakeTransform (Math|Vector|MakeVector (* _index_2 (Variables|Default|GetTileSizeX)) (* _index (Variables|Default|GetTileSizeY)) 0.0) "0, 0, 0" "1.000000,1.000000,1.000000") false)
      (if (Variables|Default|GetRoofTop?)
        (Components|InstancedStaticMesh|AddInstance (Variables|Default|GetCelling) (Math|Transform|MakeTransform (+ (Math|Vector|MakeVector (* _index_2 (Variables|Default|GetTileSizeX)) (* _index (Variables|Default|GetTileSizeY)) 0.0) (Math|Vector|MakeVector 0.0 0.0 (Variables|Default|GetTileSizeZ))) "0, 0, 0" "1.000000,1.000000,1.000000") false))))
  (for _index_3 (range 0 (- (Variables|Default|GetRoomTileY) 1))
    (CallFunction|WallorDoor (Math|Vector|MakeVector 0.0 (* (Variables|Default|GetTileSizeY) _index_3) 0.0) "0, 0, 0" (== (Math|Integer|%(Integer) _index_3 (Variables|Default|GetDoorEvery)) (Variables|Default|GetDoorReminder)))
    (CallFunction|WallorDoor (Math|Vector|MakeVector (* (Variables|Default|GetRoomTileX) (Variables|Default|GetTileSizeX)) (* (Variables|Default|GetTileSizeY) (- _index_3 1)) 0.0) "0.000000,180.000000,0.000000" (== (Math|Integer|%(Integer) _index_3 (Variables|Default|GetDoorEvery)) (Variables|Default|GetDoorReminder))))
  (for _index_4 (range 0 (- (Variables|Default|GetRoomTileX) 1))
    (CallFunction|WallorDoor (Math|Vector|MakeVector (* (Variables|Default|GetTileSizeX) _index_4) (* (Variables|Default|GetTileSizeY) (- (Variables|Default|GetRoomTileY) 1)) 0.0) "0.000000,90.000000,0.000000" (== (Math|Integer|%(Integer) _index_4 (Variables|Default|GetDoorEvery)) (Variables|Default|GetDoorReminder)))
    (CallFunction|WallorDoor (Math|Vector|MakeVector (* (Variables|Default|GetTileSizeX) (+ _index_4 1.0)) (* (Variables|Default|GetTileSizeY) -1.0) 0.0) "0.000000,-90.000000,0.000000" (== (Math|Integer|%(Integer) _index_4 (Variables|Default|GetDoorEvery)) (Variables|Default|GetDoorReminder)))))

(fn WallorDoor
  (params (Instance%20Transform%20Location :type Vector) (Instance%20Transform%20Rotation :type Rotator) (CanDoor :type Boolean))
  (bind _returnvalue (Transformation|GetActorTransform))
  (bind _doorcount (Variables|Default|GetDoorCount))
  (if (and CanDoor (Class|KismetMathLibrary|RandomBoolwithWeightfromStream (Variables|Default|GetRoomStream) (Math|Conversions|ToFloat(Integer) (/ _doorcount (- _doorcount (Utilities|Array|Length (Variables|Default|GetDoors)))))))
    (bind _returnvalue_2 (Game|SpawnActorfromClass "/Game/BluePrint/ProceduralContent/Door.Door_C" (Math|Transform|MakeTransform (Math|Transform|TransformLocation _returnvalue Instance%20Transform%20Location) (Math|Transform|TransformRotation _returnvalue Instance%20Transform%20Rotation) "1.000000,1.000000,1.000000") "AlwaysSpawn" "MultiplyWithRoot" 0 0))
    (Utilities|Array|Add (Variables|Default|GetDoors) _returnvalue_2)
    (else
      (Components|InstancedStaticMesh|AddInstance (Variables|Default|GetWall) (Math|Transform|MakeTransform Instance%20Transform%20Location Instance%20Transform%20Rotation "1.000000,1.000000,1.000000") false))))